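; Collectable story pickup that shows a sprite on a plane, with the material applied in the construction script.
; When a TenticleController component whose first tag is "TenticleBone" overlaps the box, it fires once and forces left-mouse release on the controller.
; It then has the controller create a dialogue widget from its story text and UI sprite, passing a camera-return flag.
; A timeline then fades out its RectLight from the starting intensity.
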(event OnComponentBeginOverlap(Box)
  (params (OverlappedComponent :type Primitive%20Component%20Object%20Reference) (OtherActor :type Actor%20Object%20Reference) (OtherComp :type Primitive%20Component%20Object%20Reference) (OtherBodyIndex :type Integer) (bFromSweep :type Boolean) (SweepResult :type Hit%20Result%20Structure%20%28by%20ref%29))
  (bind _astenticle_controller (Utilities|Casting|CastToTenticleController OtherActor))
  (if (== (Utilities|Array|Get(acopy) (Variables|/Script/Engine.ActorComponent|GetComponentTags OtherComp)) "TenticleBone")
    (Utilities|FlowControl|DoOnce false
      (:Completed
        (Default|CEForceLeftMouseReleased _astenticle_controller)
        (Default|CECreateScreenWidget _astenticle_controller (Variables|Default|GetStoryBlockContents) (Variables|Default|GetM_AssetSprite_UI) (Variables|Default|GetReturnCameraOnCollected))
        ;[1 1 1] Turn off the ligth
        (Variables|Default|SetStartingIntensity (Variables|/Script/Engine.LightComponentBase|GetIntensity (Variables|Default|GetRectLight)))
        (bind _fadeoutlight (Timeline|FadeOutTheRectLight PlayFromStart)
          (:Update
            (Rendering|Components|Light|SetIntensity (Variables|Default|GetRectLight) (Math|Float|Lerp 0.0 (Variables|Default|GetStartingIntensity) _fadeoutlight))))))))

(event EventBeginPlay)

(event Collision|EventActorBeginOverlap
  (params (OtherActor :type Actor%20Object%20Reference)))

(event EventTick
  (params (DeltaSeconds :type Float%20%28single-precision%29)))

(fn ConstructionScript
  (Rendering|Material|SetMaterial (Variables|Default|GetPlane) 0 (Variables|Default|GetM_AssetSprite)))